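; Test Blueprint for a destructible object that the player smashes by right-clicking it at close range.
; It binds to the RageController right-click event and uses cursor hover to arm a flag while the object can still be damaged.
; A valid click plays the character's attack animation, applies damage and impulse after a delay, disables re-arming, then restores Animation Blueprint mode.
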(event `self.ReceiveBeginPlay`
  (add `/Game/Rage/Blueprints/RageController.RightClickPressedEvdent` (cast `/Game/Rage/Blueprints/RageController` (`GameplayStatics.GetPlayerController` 0) :!pure true) (delegate `MouseRight`))
  (set `self.canbedamage` true))

(event `MouseRight`
  (bind _returnvalue (`self.K2_GetActorLocation` self))
  (bind _mesh (`Character.Mesh` (cast `/Game/Rage/Blueprints/RageCharacter` (`GameplayStatics.GetPlayerCharacter` 0) :!pure true)))
  (if (`self.test`)
    ;[1 1 1] destructible right click test
    (if (< (`self.GetDistanceTo` (`GameplayStatics.GetPlayerCharacter` 0) self) 200.0)
      (`SkeletalMeshComponent.PlayAnimation` _mesh "/Game/InfinityBladeWarriors/Character/Animations/Attack.Attack" false)
      (`KismetSystemLibrary.Delay` 0.5)
      (`DestructibleComponent.ApplyDamage` (`self.Destructible`) 300.0 _returnvalue _returnvalue 3000.0)
      (set `self.canbedamage` false)
      (`KismetSystemLibrary.Delay` 0.8)
      (`SkeletalMeshComponent.SetAnimationMode` _mesh "AnimationBlueprint"))))

(event `self.Destructible.OnBeginCursorOver`
  (params (TouchedComponent :type "PrimitiveComponent Object Reference"))
  (if (`self.canbedamage`)
    (set `self.test` true)))

(event `self.ReceiveActorEndCursorOver`
  (set `self.test` false))

(fn `UserConstructionScript`)