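; AI controller that drives an EnnemyCharacter to chase and attack the first player's character.
; Each tick, while the pawn's PV is above zero, it yaws the pawn toward the player and issues a simple move-to toward them.
; A distance check sets the IsAttacking flag on AttackComponent when the player is within close range and clears it otherwise.
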(event `self.ReceiveTick`
  (params (DeltaSeconds :type "Float (single-precision)"))
  (bind _returnvalue (`GameplayStatics.GetPlayerCharacter` 0))
  (bind _attackcomponent (`self.AttackComponent`))
  (bind _asennemy_character (cast `/Game/Rage/Blueprints/EnnemyCharacter` (`self.K2_GetPawn`) :!pure true))
  (bind (_returnvalue_roll _returnvalue_pitch _returnvalue_yaw) (`KismetMathLibrary.BreakRotator` (`KismetMathLibrary.FindLookAtRotation` (`self.K2_GetActorLocation` _asennemy_character) (`self.K2_GetActorLocation` (`GameplayStatics.GetPlayerCharacter` 0)))))
  (if (> (`KismetMathLibrary.Conv_IntToDouble` (`/Game/Rage/Blueprints/EnnemyCharacter.PV` _asennemy_character)) 0.0)
    (`self.K2_SetActorRotation` _asennemy_character (`KismetMathLibrary.MakeRotator` 0.0 0.0 _returnvalue_yaw) false)
    (`NavigationSystem.SimpleMoveToActor` (`AIBlueprintHelperLibrary.GetAIController` self) _returnvalue)
    (if (<= (`self.GetDistanceTo` _asennemy_character _returnvalue) 150.0)
      (set `/Game/Rage/Blueprints/AttackComponent.isAttacking` true _attackcomponent)
      (else
        (set `/Game/Rage/Blueprints/AttackComponent.isAttacking` false _attackcomponent)))))

(fn `UserConstructionScript`)