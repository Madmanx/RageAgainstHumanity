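; Enemy character with hit points (PV) shown on a PvEnnemyBar widget component.
; Any damage taken is subtracted from PV and pushed to the bar, whose maximum is set from PV at BeginPlay.
; Hovering the capsule switches the mouse cursor to a slashed circle.
; Tick watches for PV at or below zero, then once enables capsule physics and launches it upward with a large impulse.
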(event `self.ReceiveBeginPlay`
  (add `self.OnTakeAnyDamage` (delegate `OnTakeAnyDamage_Event_0`))
  (set `/Game/Rage/Widget/PvEnnemyBar.MaxPv` (`KismetMathLibrary.Conv_IntToDouble` (`self.PV`)) (cast `/Game/Rage/Widget/PvEnnemyBar` (`WidgetComponent.GetUserWidgetObject` (`self.Widget`)) :!pure true)))

(event `OnTakeAnyDamage_Event_0` :!signature `self.OnTakeAnyDamage`
  (params (DamagedActor :type "Actor Object Reference") (Damage :type "Float (double-precision)") (DamageType :type "DamageType Object Reference") (InstigatedBy :type "Controller Object Reference") (DamageCauser :type "Actor Object Reference"))
  (bind _output_get (set `self.PV` (`KismetMathLibrary.FTrunc` (- (`KismetMathLibrary.Conv_IntToDouble` (`self.PV`)) Damage))))
  (set `/Game/Rage/Widget/PvEnnemyBar.Pv` (`KismetMathLibrary.Conv_IntToDouble` _output_get) (cast `/Game/Rage/Widget/PvEnnemyBar` (`WidgetComponent.GetUserWidgetObject` (`self.Widget`)) :!pure true)))

(event `self.CapsuleComponent.OnBeginCursorOver`
  (params (TouchedComponent :type "PrimitiveComponent Object Reference"))
  (set `PlayerController.CurrentMouseCursor` "SlashedCircle" (`GameplayStatics.GetPlayerController` 0)))

(event `self.CapsuleComponent.OnEndCursorOver`
  (params (TouchedComponent :type "PrimitiveComponent Object Reference"))
  (set `PlayerController.CurrentMouseCursor` "Default" (`GameplayStatics.GetPlayerController` 0)))

(event `self.ReceiveTick`
  (params (DeltaSeconds :type "Float (single-precision)"))
  (bind _capsulecomponent (`self.CapsuleComponent`))
  (if (<= (`self.PV`) 0)
    (`/Engine/EditorBlueprintResources/StandardMacros.DoOnce` false
      (:`Completed`
        (`PrimitiveComponent.SetSimulatePhysics` _capsulecomponent true)
        (`PrimitiveComponent.AddImpulseAtLocation` _capsulecomponent (0.0 0.0 500000.0) (`SceneComponent.K2_GetComponentLocation` _capsulecomponent) "None")))))

(fn `UserConstructionScript`)