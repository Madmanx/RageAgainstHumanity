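; Consumable pickup actor that the player clicks on the ground to add a potion to the inventory.
; On BeginPlay it rescales itself and fills its tooltip widget with its name.
; While on the ground, mouse hover toggles the tooltip and swaps the cursor.
; Clicking creates a potion item widget in the first empty slot of the RageHud inventory, then destroys the actor and resets the cursor.
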(event `self.ReceiveBeginPlay`
  (`self.SetActorScale3D` (0.25 0.25 0.7))
  (`/Game/Rage/Widget/Tooltip_Widget_UI.Init` (cast `/Game/Rage/Widget/Tooltip_Widget_UI` (`WidgetComponent.GetUserWidgetObject` (`self.Widget`)) :!pure true) (`self.Name`) 70.0 false))

(event `self.StaticMesh.OnBeginCursorOver`
  (params (TouchedComponent :type "PrimitiveComponent Object Reference"))
  (if (`self.isOnGround`)
    (`SceneComponent.SetVisibility` (`self.Widget`) true false)
    (set `PlayerController.CurrentMouseCursor` "GrabHand" (`GameplayStatics.GetPlayerController` 0))))

(event `self.StaticMesh.OnEndCursorOver`
  (params (TouchedComponent :type "PrimitiveComponent Object Reference"))
  (if (`self.isOnGround`)
    (`SceneComponent.SetVisibility` (`self.Widget`) false false)
    (set `PlayerController.CurrentMouseCursor` "Crosshairs" (`GameplayStatics.GetPlayerController` 0))))

(event `self.StaticMesh.OnClicked`
  (params (TouchedComponent :type "PrimitiveComponent Object Reference") (ButtonPressed :type "Key Structure"))
  (bind _itemslots (`/Game/Inventory/Widgets/Inventoty_UI.ItemSlots` (`/Game/Rage/Widget/RageHud.Inventory_Ref` (cast `/Game/Rage/Widget/RageHud` (`PlayerController.GetHUD` (`GameplayStatics.GetPlayerController` 0)) :!pure true))))
  ;[0 0.1472 1] Add item potion$
  (for _index (range (+ (`KismetArrayLibrary.Array_Length` _itemslots) 1))
    (bind _output (`|GetArrayItem` _itemslots _index))
    (`/Engine/EditorBlueprintResources/StandardMacros.IsValid` (`/Game/Inventory/Widgets/ItemSlot_UI.ItemInThisSlot` _output)
      (:`Is Not Valid`
        (bind _returnvalue (`|CreateWidget` "/Game/Inventory/Widgets/ItemWidget_UI.ItemWidget_UI_C"))
        (`/Game/Inventory/Widgets/ItemWidget_UI.CreatePotion` _returnvalue)
        (`/Game/Inventory/Widgets/ItemSlot_UI.AddItemToThisSlot` _output _returnvalue)
        (`self.K2_DestroyActor`)
        (set `PlayerController.CurrentMouseCursor` "Crosshairs" (`GameplayStatics.GetPlayerController` 0))
        (break)))))

(fn `UserConstructionScript`)